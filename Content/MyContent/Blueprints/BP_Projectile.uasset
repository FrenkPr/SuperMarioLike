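; BP_Projectile is a fiery projectile that flies at the player and explodes on impact.
; On BeginPlay it locks a direction toward the player pawn's current position, without homing afterward, and attaches a fire particle effect.
; Tick moves it along that direction at Speed with a swept SetActorLocation.
; A mesh hit on any valid actor spawns an explosion and destroys the projectile, applying damage only to actors tagged Player.
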(event `self.ReceiveBeginPlay`
  (set `self.Direction` (`KismetMathLibrary.Normal` (- (`self.K2_GetActorLocation` (`GameplayStatics.GetPlayerPawn` 0)) (`self.K2_GetActorLocation`))))
  (`GameplayStatics.SpawnEmitterAttached` "/Game/StarterContent/Particles/P_Fire.P_Fire" (`self.StaticMesh`) "None" (0.0 0.0 0.0) (struct) (1.0 1.0 1.0) "SnapToTarget"))

(event `self.ReceiveTick`
  (params (DeltaSeconds :type "Float (single-precision)"))
  (`self.K2_SetActorLocation` (+ (`self.K2_GetActorLocation`) (* (`self.Direction`) (* DeltaSeconds (`self.Speed`)))) true))

(event `self.StaticMesh.OnComponentHit`
  (params (HitComponent :type "PrimitiveComponent Object Reference") (OtherActor :type "Actor Object Reference") (OtherComp :type "PrimitiveComponent Object Reference") (NormalImpulse :type "Vector Structure") (Hit :type "HitResult Structure (by ref)"))
  (`/Engine/EditorBlueprintResources/StandardMacros.IsValid` OtherActor
    (:`Is Valid`
      (if (`self.ActorHasTag` OtherActor "Player")
        (`GameplayStatics.ApplyDamage` OtherActor 100.0))
      (`GameplayStatics.SpawnEmitterAtLocation` "/Game/StarterContent/Particles/P_Explosion.P_Explosion" (`.ImpactPoint` (`GameplayStatics.BreakHitResult` Hit)))
      (`self.K2_DestroyActor`))))

(fn `UserConstructionScript`)