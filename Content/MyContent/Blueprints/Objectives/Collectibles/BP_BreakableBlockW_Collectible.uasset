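; BP_BreakableBlockW_Collectible is a breakable block child Blueprint meant to release a collectible when the player hits it from below.
; Its graph checks the Player tag and impact normal, spawns a half-scale, physics-simulated BP_Collectible above the block, then destroys the block.
; That logic is unconnected to any event, so it never runs here; the construction script only calls the parent.
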(fn `UserConstructionScript`
  (`parent.UserConstructionScript`))