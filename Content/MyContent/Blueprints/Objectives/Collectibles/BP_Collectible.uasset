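; BP_Collectible is a pickup that the player collects by walking into it.
; When its Collectible component overlaps an actor tagged Player, it destroys itself and then tells the HUD widget to update the collectibles count.
; A helper function finds that HUD by casting the first player character to ThirdPersonCharacter, printing a message if the cast fails.
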(event `self.Collectible.OnComponentBeginOverlap`
  (params (OverlappedComponent :type "PrimitiveComponent Object Reference") (OtherActor :type "Actor Object Reference") (OtherComp :type "PrimitiveComponent Object Reference") (OtherBodyIndex :type Integer) (bFromSweep :type Boolean) (SweepResult :type "HitResult Structure (by ref)"))
  (if (`self.ActorHasTag` OtherActor "Player")
    (`self.K2_DestroyActor`)
    (`/Game/MyContent/Blueprints/HUD/WBP_HUD.UpdateCollectiblesCount` (`self.GetHUD`))))

(fn `GetHUD`
  (returns (HUD :type "/Game/MyContent/Blueprints/HUD/WBP_HUD Object Reference"))
  (bind _asthird_person_character (cast `/Game/MyContent/Blueprints/ThirdPersonCharacter` (`GameplayStatics.GetPlayerCharacter` 0))
    (:`then`
      _)
    (:`CastFailed`
      (`KismetSystemLibrary.PrintString` "ThirdPersonCharacter cast failed")))
  (return (`/Game/MyContent/Blueprints/ThirdPersonCharacter.GetWBP_HUD` _asthird_person_character)))

(fn `UserConstructionScript`)