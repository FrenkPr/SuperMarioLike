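; BP_ArenaVolume is an arena trigger volume that registers the objectives inside it with a BPObjectiveTarget and counts them.
; Shortly after BeginPlay it moves the volume to TargetPosition, forcing begin-overlap events for objectives already in the arena.
; Overlapping actors tagged "Objective" increment NumObjectives and receive the target reference, set on collectibles (when included) or on an enemy's objective.
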(event `self.ReceiveBeginPlay`
  ;[1 1 1] We move the volume into the arena location to let overlap every objective with it at start game or OnBeginOverlap event won't be called.
  (`KismetSystemLibrary.Delay` 0.1)
  (`SceneComponent.K2_SetWorldLocation` (`self.ArenaVolume`) (`self.TargetPosition`) false false))

(event `self.ArenaVolume.OnComponentBeginOverlap`
  (params (OverlappedComponent :type "PrimitiveComponent Object Reference") (OtherActor :type "Actor Object Reference") (OtherComp :type "PrimitiveComponent Object Reference") (OtherBodyIndex :type Integer) (bFromSweep :type Boolean) (SweepResult :type "HitResult Structure (by ref)"))
  ;[1 1 1] Checks if there are objectives to complete
  (if (`self.ActorHasTag` OtherActor "Objective")
    (if (`self.IncludeCollectiblesAsObjective?`)
      ;;[1 0.5785 0] Here means it found a collectible as objective
      (bind _asbp_objective (cast `/Game/MyContent/Blueprints/Objectives/BP_Objective` OtherActor)
        (:`then`
          (set `/Game/MyContent/Blueprints/Objectives/BP_Objective.BP_ObjectiveTarget` (`self.BP_ObjectiveTarget`) _asbp_objective))
        (:`CastFailed`
          ;;[1 0 0.000951] Here means it found an enemy as objective
          (bind _asbp_enemy (cast `/Game/MyContent/Blueprints/Objectives/Enemies/BP_Enemy` OtherActor :!label _label))
          (bind _bp_objective (`/Game/MyContent/Blueprints/Objectives/Enemies/BP_Enemy.BP_Objective` _asbp_enemy)
            (:`then`
              (set `/Game/MyContent/Blueprints/Objectives/BP_Objective.BP_ObjectiveTarget` (`self.BP_ObjectiveTarget`) _bp_objective))
            (:`else`))))
      (else
        (goto _label)))
    (`/Engine/EditorBlueprintResources/StandardMacros.IncrementInt` (`/Game/MyContent/Blueprints/Door/BP_DoorW_Objective.NumObjectives` (`self.BP_ObjectiveTarget`)))))

(fn `UserConstructionScript`)