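; BP_BossFightStartCollider is a trigger actor that starts the boss fight when a Player-tagged actor first overlaps its collider.
; A timed sequence locks player input, calls EnableInvincibility on the boss, restores input, then starts the fight music and hands the sound to the boss.
; It then switches the boss AI controller's behavior tree state to shoot the player and destroys itself.
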(event `self.BossFightStartCollider.OnComponentBeginOverlap`
  (params (OverlappedComponent :type "PrimitiveComponent Object Reference") (OtherActor :type "Actor Object Reference") (OtherComp :type "PrimitiveComponent Object Reference") (OtherBodyIndex :type Integer) (bFromSweep :type Boolean) (SweepResult :type "HitResult Structure (by ref)"))
  (if (and (`self.ActorHasTag` OtherActor "Player") (not (`self.BossFightActivated?`)))
    (`self.StartBossFight`)))

(event `StartBossFight`
  (bind _bp_boss (`self.BP_Boss`))
  (set `self.BossFightActivated?` true)
  (`self.DisableInput` (`self.BP_Player`) (`GameplayStatics.GetPlayerController` 0))
  (`KismetSystemLibrary.Delay` 2.0)
  (`/Game/MyContent/Blueprints/Objectives/Enemies/BP_Enemy.EnableInvincibility` (`self.BP_Boss`))
  (`KismetSystemLibrary.Delay` 1.0)
  (`self.EnableInput` (`self.BP_Player`) (`GameplayStatics.GetPlayerController` 0))
  (`KismetSystemLibrary.Delay` 2.0)
  (bind _returnvalue (`GameplayStatics.SpawnSound2D` "/Game/MyContent/Sounds/BuiltToFallBossFight.BuiltToFallBossFight" 1.0 1.0 0.0 null false false))
  (set `/Game/MyContent/Blueprints/Objectives/Enemies/BP_Boss.SFX_BossFight` _returnvalue _bp_boss)
  (bind _asbp_boss_ctrl (cast `/Game/MyContent/Blueprints/Objectives/Enemies/AI/Controllers/BP_BossCtrl` (`AIBlueprintHelperLibrary.GetAIController` _bp_boss))
    (:`then`
      (`/Game/MyContent/Blueprints/Objectives/Enemies/AI/Controllers/BP_BossCtrl.SetBT_StateToShootPlayer` _asbp_boss_ctrl)
      (`self.K2_DestroyActor`))
    (:`CastFailed`
      (`KismetSystemLibrary.PrintString` "Cast to BP_BossCtrl failed"))))

(fn `UserConstructionScript`)