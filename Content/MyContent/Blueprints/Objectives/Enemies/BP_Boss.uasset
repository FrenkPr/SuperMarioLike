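; Boss enemy that the player hurts by jumping on its head; most other contact damages the player, except landing on the arms.
; A head stomp grants invincibility and restarts the BP_BossCtrl timer for switching its behavior tree to shooting.
; On destruction it spawns BP_EndGame and stops the fight audio.
; Helper functions show or hide cloud platforms along with their collision.
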(event `self.CapsuleComponent.OnComponentHit`
  (params (HitComponent :type "PrimitiveComponent Object Reference") (OtherActor :type "Actor Object Reference") (OtherComp :type "PrimitiveComponent Object Reference") (NormalImpulse :type "Vector Structure") (Hit :type "HitResult Structure (by ref)"))
  ;[1 1 1] To fix BP_Projectile exception
  (`/Engine/EditorBlueprintResources/StandardMacros.IsValid` OtherActor
    (:`Is Valid`
      (if (`self.ActorHasTag` OtherActor "Player")
        (`GameplayStatics.ApplyDamage` (`GameplayStatics.GetPlayerCharacter` 0) 100.0)))))

(event `self.ArmsCapsuleCollider.OnComponentHit`
  (params (HitComponent :type "PrimitiveComponent Object Reference") (OtherActor :type "Actor Object Reference") (OtherComp :type "PrimitiveComponent Object Reference") (NormalImpulse :type "Vector Structure") (Hit :type "HitResult Structure (by ref)"))
  ;[1 1 1] To fix BP_Projectile exception
  (`/Engine/EditorBlueprintResources/StandardMacros.IsValid` OtherActor
    (:`Is Valid`
      (if (`self.ActorHasTag` OtherActor "Player")
        (if (not (< (.z Hit_ImpactNormal) 0.0))
          (`GameplayStatics.ApplyDamage` (`GameplayStatics.GetPlayerCharacter` 0) 100.0))))))

(event `self.HeadCapsuleCollider.OnComponentHit`
  (params (HitComponent :type "PrimitiveComponent Object Reference") (OtherActor :type "Actor Object Reference") (OtherComp :type "PrimitiveComponent Object Reference") (NormalImpulse :type "Vector Structure") (Hit :type "HitResult Structure (by ref)"))
  ;[1 1 1] To fix BP_Projectile exception
  (`/Engine/EditorBlueprintResources/StandardMacros.IsValid` OtherActor
    (:`Is Valid`
      (if (`self.ActorHasTag` OtherActor "Player")
        (if (and (< (.z Hit_ImpactNormal) 0.0) (not (`NavMovementComponent.IsMovingOnGround` (`Character.CharacterMovement` (`GameplayStatics.GetPlayerCharacter` 0)))))
          (`GameplayStatics.ApplyDamage` self 100.0)
          (`self.EnableInvincibility`)
          (bind _asbp_boss_ctrl (cast `/Game/MyContent/Blueprints/Objectives/Enemies/AI/Controllers/BP_BossCtrl` (`AIBlueprintHelperLibrary.GetAIController` self)))
          (`KismetSystemLibrary.K2_ClearAndInvalidateTimerHandle` (`/Game/MyContent/Blueprints/Objectives/Enemies/AI/Controllers/BP_ShooterEnemyCtrl.ShootPlayerTimer` _asbp_boss_ctrl))
          (bind _returnvalue (`KismetSystemLibrary.K2_SetTimer` _asbp_boss_ctrl "SetBT_StateToShootPlayer" 2.0))
          (set `/Game/MyContent/Blueprints/Objectives/Enemies/AI/Controllers/BP_ShooterEnemyCtrl.ShootPlayerTimer` _returnvalue _asbp_boss_ctrl)
          (else
            (`GameplayStatics.ApplyDamage` (`GameplayStatics.GetPlayerCharacter` 0) 100.0)))))))

(event `self.ReceiveDestroyed`
  (`parent.ReceiveDestroyed`)
  (`|SpawnActorFromClass` "/Game/MyContent/Blueprints/BP_EndGame.BP_EndGame_C" (`KismetMathLibrary.MakeTransform` (- (`self.K2_GetActorLocation`) (0.0 0.0 15.0)) (struct :`Yaw` -90.0) (0.75 7.75 3.75)) "Undefined" "OverrideRootScale" null null)
  (`self.StopSound2D` (`self.SFX_BossFight`)))

(fn `DisablePlatforms`
  (for _array_element (`self.BP_CloudPlatforms`)
    (`PrimitiveComponent.SetCollisionProfileName` (`/Game/MyContent/Blueprints/Platforms/BP_CloudPlatform.Platform` _array_element) "NoCollision" true)
    (`PrimitiveComponent.SetCollisionProfileName` (`/Game/MyContent/Blueprints/Platforms/BP_CloudPlatform.CloudBoxOverlapper` _array_element) "NoCollision" true)
    (`SceneComponent.SetVisibility` (`/Game/MyContent/Blueprints/Platforms/BP_CloudPlatform.Platform` _array_element) false false)))

(fn `EnablePlatforms`
  (for _array_element (`self.BP_CloudPlatforms`)
    (`PrimitiveComponent.SetCollisionProfileName` (`/Game/MyContent/Blueprints/Platforms/BP_CloudPlatform.Platform` _array_element) "BlockAll" true)
    (`PrimitiveComponent.SetCollisionProfileName` (`/Game/MyContent/Blueprints/Platforms/BP_CloudPlatform.CloudBoxOverlapper` _array_element) "OverlapAllDynamic" true)
    (`SceneComponent.SetVisibility` (`/Game/MyContent/Blueprints/Platforms/BP_CloudPlatform.Platform` _array_element) true false)))

(fn `StopSound2D`
  (params (AudioComponent :type "AudioComponent Object Reference"))
  (`/Engine/EditorBlueprintResources/StandardMacros.IsValid` AudioComponent
    (:`Is Valid`
      (`AudioComponent.Stop` AudioComponent))
    (:`Is Not Valid`
      _))
  (return))

(fn `UserConstructionScript`
  (`parent.UserConstructionScript`))