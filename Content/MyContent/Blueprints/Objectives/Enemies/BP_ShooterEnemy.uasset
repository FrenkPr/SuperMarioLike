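; Shooter enemy Blueprint that fires BP_Projectile actors from an offset around its own location.
; BeginPlay runs the parent logic, then unrotates ShootOffset by the mesh's relative rotation.
; Shoot spawns a scaled-down projectile, multiplying the offset's X and Y component-wise by the actor's forward vector rather than rotating it, and passes no spawn rotation.
; No call to Shoot appears within this Blueprint.
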(event `self.ReceiveBeginPlay`
  (`parent.ReceiveBeginPlay`)
  (set `self.ShootOffset` (`KismetMathLibrary.LessLess_VectorRotator` (`self.ShootOffset`) (`SceneComponent.RelativeRotation` (`self.Mesh`)))))

(fn `Shoot`
  (bind (_returnvalue_x _returnvalue_y) (`KismetMathLibrary.BreakVector` (`self.GetActorForwardVector`)))
  (`|SpawnActorFromClass` "/Game/MyContent/Blueprints/BP_Projectile.BP_Projectile_C" (`KismetMathLibrary.MakeTransform` (+ (`self.K2_GetActorLocation`) (* (`self.ShootOffset`) (`KismetMathLibrary.MakeVector` _returnvalue_x _returnvalue_y 1.0))) (struct) (0.1 0.1 0.1)) "Undefined" "OverrideRootScale" null null))

(fn `UserConstructionScript`
  (`parent.UserConstructionScript`))