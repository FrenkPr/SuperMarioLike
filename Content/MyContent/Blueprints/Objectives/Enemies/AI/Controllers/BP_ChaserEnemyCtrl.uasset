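; AI controller for chaser enemies that runs BT_ChaserEnemy on a possessed BP_Enemy and stores the player as its Blackboard target.
; Perception sets HasLineOfSight and starts a looping timer that pushes the enemy toward a nearby player with swept teleports to force collision.
; When sight is lost and the player is grounded, a delayed timer clears line of sight and stops the push, so jumping does not break the chase.
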(event `self.ReceiveBeginPlay`
  (`BlackboardComponent.SetValueAsObject` (`self.Blackboard`) (`self.PlayerTarget`) (`GameplayStatics.GetPlayerCharacter` 0)))

(event `self.ReceivePossess`
  (params (PossessedPawn :type "Pawn Object Reference"))
  (bind _asbp_enemy (cast `/Game/MyContent/Blueprints/Objectives/Enemies/BP_Enemy` PossessedPawn)
    (:`then`
      (set `self.Possessed Pawn` _asbp_enemy)
      (`self.RunBehaviorTree` "/Game/MyContent/Blueprints/Objectives/Enemies/AI/BehavoiurTrees/BT_ChaserEnemy.BT_ChaserEnemy"))
    (:`CastFailed`
      (`KismetSystemLibrary.PrintString` "Cast to BP_Enemy failed"))))

(event `LetTheEnemyCollideWithPlayer`
  (bind _possessed_pawn (`self.Possessed Pawn`))
  (bind _possessed_pawn_2 (`self.Possessed Pawn`))
  (bind _returnvalue (- (`self.K2_GetActorLocation` (`GameplayStatics.GetPlayerCharacter` 0)) (`self.K2_GetActorLocation` _possessed_pawn)))
  ;[1 1 1] Enemy can see player
  (if (<= (`KismetMathLibrary.VSize` _returnvalue) (`/Game/MyContent/Blueprints/Objectives/Enemies/BP_Enemy.CollisionDistance` _possessed_pawn))
    (`self.K2_SetActorLocation` _possessed_pawn_2 (+ (`self.K2_GetActorLocation` _possessed_pawn_2) (* (`KismetMathLibrary.Normal` _returnvalue) (`CharacterMovementComponent.MaxWalkSpeed` (`Character.CharacterMovement` _possessed_pawn_2)))) true true)))

(event `self.AIPerception.OnTargetPerceptionUpdated`
  (params (Actor :type "Actor Object Reference") (Stimulus :type "AIStimulus Structure"))
  ;[1 1 1] Checks if the player is in the
  ; enemy's sight
  (if (and (`self.ActorHasTag` Actor "Player") Stimulus_bSuccessfullySensed (`self.ActorHasTag` "ChaserEnemyCtrl"))
    ;[1 1 1] Enemy can see player
    (`KismetSystemLibrary.K2_ClearAndInvalidateTimerHandle` (`self.ResetBB_ValuesOnPatrolTimer`))
    (`BlackboardComponent.SetValueAsBool` (`self.Blackboard`) (`self.HasLineOfSight`) true)
    (bind _returnvalue (`KismetSystemLibrary.K2_SetTimerDelegate` (delegate `LetTheEnemyCollideWithPlayer`) 0.1 true))
    (set `self.LetTheEnemyCollideWithPlayerTimer` _returnvalue)
    (else
      ;[1 1 1] Enemy can't see player
      ;;[1 1 1] Won't let the enemy lose the player as target while the player is jumping and is near to the enemy
      (bind _asthird_person_character (cast `/Game/MyContent/Blueprints/ThirdPersonCharacter` Actor))
      (if (`NavMovementComponent.IsMovingOnGround` (`Character.CharacterMovement` _asthird_person_character))
        (bind _returnvalue_2 (`KismetSystemLibrary.K2_SetTimerDelegate` (delegate `GoToPatrol`) (`self.FromChaseToPatrolTime`)))
        (set `self.ResetBB_ValuesOnPatrolTimer` _returnvalue_2)))))

(event `GoToPatrol`
  ;[1 1 1] Enemy can't see player
  (`BlackboardComponent.SetValueAsBool` (`self.Blackboard`) (`self.HasLineOfSight`) false)
  (`KismetSystemLibrary.K2_ClearAndInvalidateTimerHandle` (`self.LetTheEnemyCollideWithPlayerTimer`)))

(fn `UserConstructionScript`)