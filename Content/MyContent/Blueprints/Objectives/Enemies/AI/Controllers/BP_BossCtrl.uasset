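; AI controller for the boss enemy that runs BT_Boss on possession and provides a timed two-phase cycle.
; Idle enables the boss platforms and clears invincibility; ShootPlayer disables them and makes it invincible, both updating the IsEnemyInvincible blackboard key.
; Each state function schedules the other by function-name timer, though nothing in this controller starts the cycle.
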(event `self.ReceivePossess`
  (params (PossessedPawn :type "Pawn Object Reference"))
  (`parent.ReceivePossess` PossessedPawn)
  (`self.RunBehaviorTree` "/Game/MyContent/Blueprints/Objectives/Enemies/AI/BehavoiurTrees/BT_Boss.BT_Boss"))

(fn `SetBT_StateToIdle`
  (bind _asbp_boss (cast `/Game/MyContent/Blueprints/Objectives/Enemies/BP_Boss` (`self.Possessed Pawn`))
    (:`then`
      (`/Game/MyContent/Blueprints/Objectives/Enemies/BP_Boss.EnablePlatforms` _asbp_boss)
      (`BlackboardComponent.SetValueAsBool` (`self.Blackboard`) (`self.IsEnemyInvincible?`) false)
      (`/Game/MyContent/Blueprints/Objectives/Enemies/BP_Enemy.DisableInvincibility` (`self.Possessed Pawn`))
      (bind _returnvalue (`KismetSystemLibrary.K2_SetTimer` null "SetBT_StateToShootPlayer" (`self.TimeToShootPlayerState`)))
      (set `self.ShootPlayerTimer` _returnvalue))
    (:`CastFailed`
      (`KismetSystemLibrary.PrintString` "Cast to BP_Boss failed"))))

(fn `SetBT_StateToShootPlayer`
  (bind _asbp_boss (cast `/Game/MyContent/Blueprints/Objectives/Enemies/BP_Boss` (`self.Possessed Pawn`))
    (:`then`
      (`/Game/MyContent/Blueprints/Objectives/Enemies/BP_Boss.DisablePlatforms` _asbp_boss)
      (`BlackboardComponent.SetValueAsBool` (`self.Blackboard`) (`self.IsEnemyInvincible?`) true)
      (`/Game/MyContent/Blueprints/Objectives/Enemies/BP_Enemy.EnableInvincibility` (`self.Possessed Pawn`))
      (`KismetSystemLibrary.K2_SetTimer` null "SetBT_StateToIdle" (`self.TimeToIdleState`)))
    (:`CastFailed`
      (`KismetSystemLibrary.PrintString` "Cast to BP_Boss failed"))))

(fn `UserConstructionScript`
  (`parent.UserConstructionScript`))