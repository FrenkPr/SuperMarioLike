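; BP_BreakableBlock is a block that the player breaks by hitting it from below to release a random collectible.
; On a component hit, it checks for the "Player" tag and an impact normal Z of exactly 1 to detect the bottom collision.
; It spawns a random pick from RandomSpawnableCollectibles above the block, enables physics on its Collectible component, and destroys itself.
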(event `self.Block.OnComponentHit`
  (params (HitComponent :type "PrimitiveComponent Object Reference") (OtherActor :type "Actor Object Reference") (OtherComp :type "PrimitiveComponent Object Reference") (NormalImpulse :type "Vector Structure") (Hit :type "HitResult Structure (by ref)"))
  (if (and (`self.ActorHasTag` OtherActor "Player") (== (.z (`.ImpactNormal` (`GameplayStatics.BreakHitResult` Hit))) 1.0))
    (bind _returnvalue (`|SpawnActorFromClass` (`KismetArrayLibrary.Array_Random` (`self.RandomSpawnableCollectibles`)) (`KismetMathLibrary.MakeTransform` (+ (`SceneComponent.K2_GetComponentLocation` (`self.Block`)) (0.0 0.0 200.0))) "Undefined" "OverrideRootScale" null null))
    (`/Engine/EditorBlueprintResources/StandardMacros.IsValid` _returnvalue
      (:`Is Valid`
        (`PrimitiveComponent.SetSimulatePhysics` (`/Game/MyContent/Blueprints/Objectives/Collectibles/BP_Collectible.Collectible` _returnvalue) true))
      (:`Is Not Valid`
        _))
    (`self.K2_DestroyActor`)))

(fn `UserConstructionScript`)