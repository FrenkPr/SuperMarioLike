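; Double door actor whose OpenDoor event swings two mesh leaves open in mirrored directions, with no closing logic.
; A timeline lerps their relative rotation from closed to plus or minus 90 degrees, chosen by the sign of GetPlayerDoorDistX, which is also printed.
; That check receives the door's own location rather than a player's, and its local-space X offset calculation is left unconnected.
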(event `OpenDoor`
  (bind _x (`self.Get_Player_Door_Dist_x` (`self.K2_GetActorLocation`)))
  (`KismetSystemLibrary.PrintString` (`KismetStringLibrary.Conv_DoubleToString` _x))
  (if (> _x 0.0)
    (set `self.OpeningRotation` (struct :`Yaw` 90.0))
    (bind (_direction _openingdoortime) (`Timeline|OpeningDoorTimeline` :!label _label)
      (:`Update`
        (bind _returnvalue (`KismetMathLibrary.RLerp` (`self.CloseningRotation`) (`self.OpeningRotation`) _openingdoortime))
        (`SceneComponent.K2_SetRelativeRotation` (`self.SM_Door1`) _returnvalue false false)
        (`SceneComponent.K2_SetRelativeRotation` (`self.SM_Door2`) (* _returnvalue -1.0) false false)))
    (else
      (set `self.OpeningRotation` (struct :`Yaw` -90.0))
      (goto _label))))

(fn `UserConstructionScript`)